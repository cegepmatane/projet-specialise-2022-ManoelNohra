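; Grappling hook actor that triggers the player character's grapple move when it hits something.
; On Hit, it casts the player character to BP_Perso, stores the character's location and the hit location as the hook's spawn and end points, then calls MoveGrapple.
; It then polls the character's movement mode through a looping short Delay and destroys itself once that mode is no longer None.
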(event `self.ReceiveHit`
  (params (MyComp :type "PrimitiveComponent Object Reference") (Other :type "Actor Object Reference") (OtherComp :type "PrimitiveComponent Object Reference") (bSelfMoved :type Boolean) (HitLocation :type "Vector Structure") (HitNormal :type "Vector Structure") (NormalImpulse :type "Vector Structure") (Hit :type "HitResult Structure (by ref)"))
  ;[1 1 1] Set up the grappling
  (bind _asbp_perso (cast `/Game/Blueprint/BP_Perso` (`GameplayStatics.GetPlayerCharacter` 0)))
  (set `Perso.HookSpawnLocation` (`self.K2_GetActorLocation` _asbp_perso) _asbp_perso)
  (set `Perso.HookEndLocation` HitLocation _asbp_perso)
  (`/Game/Blueprint/BP_Perso.MoveGrapple` _asbp_perso)
  (`KismetSystemLibrary.Delay` 0.1 :!label _label)
  (if (`|EnumInequality` (`CharacterMovementComponent.MovementMode` (`Character.CharacterMovement` _asbp_perso)) "MOVE_None")
    (`self.K2_DestroyActor`)
    (else
      (goto _label))))

(fn `UserConstructionScript`)