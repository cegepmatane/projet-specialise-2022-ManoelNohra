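; BP_Perso is a first-person player Blueprint with a grappling hook, a slide and a crosshair HUD added on BeginPlay.
; MoveGrapple disables movement and lerps the actor between hook locations on the Grapp timeline, with a clamped distance-based play rate.
; Hook completion or cancel restores walking.
; Slide, blocked while jumping, briefly switches to flying, lowers the camera and disables capsule collision, then restores them.
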(event `InputAction|CancelHook`
  (params (Key :type "Key Structure"))
  ;[1 1 1] Cancel Hook
  (:`Pressed`
    (if (`|EnumEquality` (`CharacterMovementComponent.MovementMode` (`self.CharacterMovement`)) "MOVE_None")
      (`TimelineComponent.Stop` (`self.Grapp`))
      (`CharacterMovementComponent.SetMovementMode` (`self.CharacterMovement`) "MOVE_Walking" 0)
      (set `self.isHooking` false))))

(event `MoveGrapple`
  ;[1 1 1] Move the player
  (`TimelineComponent.SetPlayRate` (`self.Grapp`) (/ 1.0 (`KismetMathLibrary.FClamp` (- (`KismetMathLibrary.VSize` (- (`self.HookSpawnLocation`) (`self.HookEndLocation`))) 12000.0) 1.0 5.0)))
  (`CharacterMovementComponent.DisableMovement` (`self.CharacterMovement`))
  (bind (_direction _graptime) (`Timeline|Grapp` :!via `PlayFromStart`)
    (:`Update`
      (`self.K2_SetActorLocation` (`KismetMathLibrary.VLerp` (`self.HookSpawnLocation`) (`self.HookEndLocation`) _graptime)))
    (:`Finished`
      (`CharacterMovementComponent.SetMovementMode` (`self.CharacterMovement`) "MOVE_Walking" 0)
      (set `self.isHooking` false))))

(event `self.ReceiveBeginPlay`
  ;[1 1 1] Move the player
  (`self.HUD`))

(event `InputAction|Slide`
  (params (Key :type "Key Structure"))
  (bind _firstpersoncamera (`self.FirstPersonCamera`))
  (bind _firstpersoncamera_2 (`self.FirstPersonCamera`))
  (bind (_relativelocation_x _relativelocation_y) (`KismetMathLibrary.BreakVector` (`SceneComponent.RelativeLocation` _firstpersoncamera)))
  (bind (_relativelocation_x_2 _relativelocation_y_2) (`KismetMathLibrary.BreakVector` (`SceneComponent.RelativeLocation` _firstpersoncamera_2)))
  ;[1 1 1] Glissade
  (:`Pressed`
    (if (not (`self.Jumping`))
      (`CharacterMovementComponent.SetMovementMode` (`self.CharacterMovement`) "MOVE_Flying" 0)
      (`SceneComponent.K2_SetRelativeLocation` _firstpersoncamera_2 (`KismetMathLibrary.MakeVector` _relativelocation_x_2 _relativelocation_y_2 21.0) false false)
      (`PrimitiveComponent.SetCollisionEnabled` (`self.CapsuleComponent`) "NoCollision")
      (`KismetSystemLibrary.Delay` 1.0)
      (`SceneComponent.K2_SetRelativeLocation` _firstpersoncamera (`KismetMathLibrary.MakeVector` _relativelocation_x _relativelocation_y 85.0) false false)
      (`PrimitiveComponent.SetCollisionEnabled` (`self.CapsuleComponent`) "QueryAndPhysics")
      (`CharacterMovementComponent.SetMovementMode` (`self.CharacterMovement`) "MOVE_Walking" 0))))

(fn `HUD`
  (bind _returnvalue (`|CreateWidget` "/Game/Blueprint/BP_CrosshairUI.BP_CrosshairUI_C"))
  (`UserWidget.AddToPlayerScreen` _returnvalue 0))

(fn `UserConstructionScript`)